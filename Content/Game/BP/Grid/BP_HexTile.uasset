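; Hex grid tile that shows its occupation status by color and displays its path cost.
; On BeginPlay and whenever occupied, reserved or vacated, it maps the status to green for vacant, blue for reserved or red for occupied.
; The color goes through ServerSetColor to a dynamic material instance on the mesh.
; Path cost changes update the text in the CostDisplay widget component.
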(event Custom|Server%20Set%20Color
  (params (Color :type Linear%20Color%20Structure))
  (CallFunction|SetColor Color))

(event EventBeginPlay
  (Class|HexTile|SetColorbyOccupationStatus))

(event EventSetColorbyOccupationStatus
  (CallFunction|ServerSetColor (Utilities|Select :Index (Class|HexTile|GetOccupationStatus) :Vacant "(R=0.000000,G=1.000000,B=0.007441,A=1.000000)" :Reserved "(R=0.000000,G=0.022493,B=1.000000,A=1.000000)" :Occupied "(R=1.000000,G=0.000000,B=0.000000,A=1.000000)")))

(event EventOnPathCostSet
  (params (cost :type Float%20%28double-precision%29))
  (bind _aswbp_simple_text (Utilities|Casting|CastToWBP_SimpleText (UserInterface|GetWidget (Variables|Default|GetCostDisplay))))
  (Default|SetText _aswbp_simple_text (Utilities|Text|ToText(Float) cost "HalfToEven" false true 1 324 0 1)))

(fn ConstructionScript)

(fn SetColor
  (params (color :type Linear%20Color%20Structure))
  (bind _returnvalue (Rendering|Material|CreateDynamicMaterialInstance (Variables|Character|GetMesh) 0 0 "None" :!class /Script/Engine.PrimitiveComponent))
  (Rendering|Material|SetVectorParameterValue _returnvalue "Color" color :!class /Script/Engine.MaterialInstanceDynamic))

(fn OnOccupied
  (params (clockwork :type Clockwork%20Unit%20Object%20Reference))
  (Class|HexTile|SetColorbyOccupationStatus)
  (return true))

(fn OnReserved
  (params (clockwork :type Clockwork%20Unit%20Object%20Reference))
  (Class|HexTile|SetColorbyOccupationStatus)
  (return true))

(fn OnVacated
  (params (clockwork :type Clockwork%20Unit%20Object%20Reference))
  (Class|HexTile|SetColorbyOccupationStatus)
  (return true))

(fn GetColor
  (bind _returnvalue (Rendering|Material|CreateDynamicMaterialInstance (Variables|Character|GetMesh) 0 0 "None" :!class /Script/Engine.PrimitiveComponent))
  (bind _returnvalue_2 (Rendering|Material|GetVectorParameterValue _returnvalue "Color" :!class /Script/Engine.MaterialInstanceDynamic))
  (return _returnvalue_2))