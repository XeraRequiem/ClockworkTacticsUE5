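; BP_ClockworkHex is a grid hex tile that shows its occupation status as a color.
; BeginPlay and the occupied, reserved and vacated overrides refresh the color, mapping the status to white, green or blue through a dynamic material instance on the mesh.
; Debug events write a cost or arbitrary text to TextDebug.
; The targeted event is an empty stub, and a moss material assignment is left unconnected.
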(event Custom|SetTargeted
  ;[0.15 0.03765 0.09358] Status
)

(event Custom|SetDebugCost
  (params (cost :type Float%20%28double-precision%29))
  ;[0 0.09959 1] Debug
  (Rendering|Components|TextRender|SetText (Variables|Default|GetText_Debug) (Utilities|Text|ToText(Float) cost "HalfToEven" false true 1 324 0 1)))

(event EventBeginPlay
  ;[0.15 0.15 0.15 0.5] Core
  (Class|ClockworkTile|SetColorbyOccupationStatus))

(event EventSetColorbyOccupationStatus
  ;[0 0.09959 1] Debug
  (CallFunction|SetColor (Utilities|Select :Index (Class|ClockworkTile|GetOccupationStatus) :Option%200 "(R=1.000000,G=1.000000,B=1.000000,A=1.000000)" :Option%201 "(R=0.119731,G=1.000000,B=0.031161,A=1.000000)" :Option%202 "(R=0.077928,G=0.305745,B=1.000000,A=1.000000)")))

(event EventDebugonTextSet
  (params (DebugText :type String))
  ;[0 0.09959 1] Debug
  (Rendering|Components|TextRender|SetText (Variables|Default|GetText_Debug) (Utilities|Text|ToText(String) DebugText)))

(fn ConstructionScript)

(fn SetColor
  (params (color :type Linear%20Color%20Structure))
  (bind _returnvalue (Rendering|Material|CreateDynamicMaterialInstance (Variables|Character|GetMesh) 0 "/Engine/BasicShapes/BasicShapeMaterial.BasicShapeMaterial" "None" :!class /Script/Engine.PrimitiveComponent))
  (Rendering|Material|SetVectorParameterValue _returnvalue "Color" color :!class /Script/Engine.MaterialInstanceDynamic))

(fn OnOccupied
  (params (Entity :type Clockwork%20Hex%20Entity%20Object%20Reference))
  (Class|ClockworkTile|SetColorbyOccupationStatus)
  (return false))

(fn OnReserved
  (params (Entity :type Clockwork%20Hex%20Entity%20Object%20Reference))
  (Class|ClockworkTile|SetColorbyOccupationStatus)
  (return false))

(fn OnVacated
  (params (Entity :type Clockwork%20Hex%20Entity%20Object%20Reference))
  (Class|ClockworkTile|SetColorbyOccupationStatus)
  (return false))