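; Test actor for replication that periodically gives its mesh a random color.
; Tick accumulates time and, past ColorChangeRate, sends a random color through the multicast event with no authority check, then resets the timer.
; Multicast, server and client events all call SetColor, which creates a dynamic material instance and sets its Color parameter.
; The server call is left disconnected, and the client event is never called here.
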(event Custom|SetColor_Multicast
  (params (Color :type Linear%20Color%20Structure))
  (CallFunction|SetColor Color))

(event Custom|SetColor_Client
  (params (Color :type Linear%20Color%20Structure))
  (CallFunction|SetColor Color))

(event Custom|SetColor_Server
  (params (Color :type Linear%20Color%20Structure))
  (CallFunction|SetColor Color))

(event EventTick
  (params (DeltaSeconds :type Float%20%28single-precision%29))
  (bind _output_get (Variables|Default|SetdColorChangeTime (+ DeltaSeconds (Variables|Default|GetdColorChangeTime))))
  (if (> _output_get (Variables|Default|GetColorChangeRate))
    (CallFunction|SetColorMulticast (Math|Color|MakeColor (Math|Random|RandomFloat) (Math|Random|RandomFloat) (Math|Random|RandomFloat) (Math|Random|RandomFloat)))
    (Variables|Default|SetdColorChangeTime 0.0)))

(fn ConstructionScript)

(fn SetColor
  (params (Color :type Linear%20Color%20Structure))
  (bind _returnvalue (Rendering|Material|CreateDynamicMaterialInstance (Variables|Default|GetMesh) 0 0 "None" :!class /Script/Engine.PrimitiveComponent))
  (Rendering|Material|SetVectorParameterValue _returnvalue "Color" Color :!class /Script/Engine.MaterialInstanceDynamic))